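; Basic enemy character that chases the player character on sight and dies when its health runs out.
; PawnSensing sightings of an IHateYouSheriffCharacter trigger an AI MoveTo toward that target.
; Any damage lowers Health and prints a debug string; at zero, a DoOnce ragdolls the mesh and spawns death particles at the head socket.
; Death also destroys the sensing and capsule components, then removes the actor after a delay.
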(event OnSeePawn(PawnSensing)
  (params (Pawn :type Pawn%20Object%20Reference))
  ;[1 1 1] Basic Movement
  (bind _asihate_you_sheriff_character (Utilities|Casting|CastToIHateYouSheriffCharacter Pawn))
  (AI|AIMoveTo self "0, 0, 0" _asihate_you_sheriff_character 5.0 true))

(event Game|Damage|EventAnyDamage
  (params (Damage :type Float%20%28single-precision%29) (DamageType :type Damage%20Type%20Object%20Reference) (InstigatedBy :type Controller%20Object%20Reference) (DamageCauser :type Actor%20Object%20Reference))
  (bind _mesh (Variables|Character|GetMesh))
  ;[1 1 1] Damage and Health
  (Variables|Default|SetHealth (- (Variables|Default|GetHealth) Damage))
  (Development|PrintString "Hello World")
  (if (<= (Variables|Default|GetHealth) 0.0)
    (Utilities|FlowControl|DoOnce false
      (:Completed
        (Physics|SetSimulatePhysics _mesh true)
        (Game|SpawnActorfromClass "/Game/Blueprints/Particle/Death_Particles.Death_Particles_C" (Math|Conversions|ToTransform(Vector) (Transformation|GetSocketLocation _mesh "head")) "Undefined" 0 0)
        (Components|DestroyComponent (Variables|Default|GetPawnSensing))
        (Components|DestroyComponent (Variables|Collision|GetCapsuleComponent))
        (Utilities|FlowControl|Delay 2e+01)
        (Actor|DestroyActor)))))

(event EventBeginPlay)

(fn ConstructionScript)