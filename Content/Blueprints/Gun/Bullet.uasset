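; Bullet actor for the gun system that plays an attached sound on spawn and destroys itself after a capsule overlap.
; The sound is selected by TypeGun, with every weapon type using the same explosion cue.
; A gate closed at BeginPlay is reopened by a delayed Tick, arming the bullet shortly after spawn.
; Overlaps pass short delays and that gate before calling ApplyDamage, which has no target wired, and destroying the actor.
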(event OnComponentBeginOverlap(Capsule)
  (params (OverlappedComponent :type Primitive%20Component%20Object%20Reference) (OtherActor :type Actor%20Object%20Reference) (OtherComp :type Primitive%20Component%20Object%20Reference) (OtherBodyIndex :type Integer) (bFromSweep :type Boolean) (SweepResult :type Hit%20Result%20Structure%20%28by%20ref%29))
  (Utilities|FlowControl|Delay 0.2)
  (Utilities|FlowControl|Gate false
    (:Exit
      (Utilities|FlowControl|Delay 0.01)
      (Game|Damage|ApplyDamage 0 1.0 0 0 "/Script/Engine.DamageType")
      (Actor|DestroyActor))))

(event EventBeginPlay
  (Audio|SpawnSoundAttached (Utilities|Select :Index (Variables|Default|GetType_Gun) :NewEnumerator0 "/Game/StarterContent/Audio/Explosion01.Explosion01" :NewEnumerator2 "/Game/StarterContent/Audio/Explosion01.Explosion01" :NewEnumerator1 "/Game/StarterContent/Audio/Explosion01.Explosion01" :NewEnumerator3 "/Game/StarterContent/Audio/Explosion01.Explosion01" :NewEnumerator4 0) (Variables|Default|GetDefaultSceneRoot))
  (Utilities|FlowControl|Gate false) ; enters at Close
)

(event Collision|EventActorBeginOverlap
  (params (OtherActor :type Actor%20Object%20Reference)))

(event EventTick
  (params (DeltaSeconds :type Float%20%28single-precision%29))
  (Utilities|FlowControl|Delay 0.4)
  (Utilities|FlowControl|Gate false) ; enters at Open
)

(fn ConstructionScript)