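; Troll enemy AI character that chases the player with AIMoveTo, gated by alive, attacking and flinch flags.
; A looping timer measures player distance and picks random short, mid or long-range montages, setting launch force and damage ranges.
; Events handle lunges, fist collision and sphere traces that spark on player hits, without applying damage.
; Incoming damage drives health, flinch logic and death, which spawns an actor at the head socket.
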(event OnComponentBeginOverlap(RightFist)
  (params (OverlappedComponent :type Primitive%20Component%20Object%20Reference) (OtherActor :type Actor%20Object%20Reference) (OtherComp :type Primitive%20Component%20Object%20Reference) (OtherBodyIndex :type Integer) (bFromSweep :type Boolean) (SweepResult :type Hit%20Result%20Structure%20%28by%20ref%29))
  (bind _returnvalue (Game|GetPlayerCharacter 0))
  ;[1 1 1] Overlap
  (if (== OtherActor _returnvalue)
    (Utilities|Casting|CastToThirdPersonCharacter _returnvalue)))

(event OnComponentBeginOverlap(LeftFist)
  (params (OverlappedComponent :type Primitive%20Component%20Object%20Reference) (OtherActor :type Actor%20Object%20Reference) (OtherComp :type Primitive%20Component%20Object%20Reference) (OtherBodyIndex :type Integer) (bFromSweep :type Boolean) (SweepResult :type Hit%20Result%20Structure%20%28by%20ref%29))
  (bind _returnvalue (Game|GetPlayerCharacter 0))
  ;[1 1 1] Overlap
  (if (== OtherActor _returnvalue)
    (Utilities|Casting|CastToThirdPersonCharacter _returnvalue)))

(event Custom|Right_Trace
  (bind _rightfist (Variables|Default|GetRightFist))
  (bind _returnvalue (Transformation|GetWorldLocation _rightfist))
  ;[1 1 1] Right
  (bind _outhit (Collision|SphereTraceForObjects _returnvalue (+ _returnvalue (* (Math|Vector|GetForwardVector (Transformation|GetWorldRotation _rightfist)) 3e+02)) 1.5e+02 (Utilities|Array|MakeArray "ObjectTypeQuery3") false 0 "None"))
  (if (== (.HitActor (Collision|BreakHitResult _outhit)) (Game|GetPlayerCharacter 0))
    (bind _returnvalue_2 (Effects|SpawnEmitteratLocation "/Game/Enemies/Blueprints/Anim_Montage_2/P_Spark.P_Spark" (.Location (Collision|BreakHitResult _outhit))))
    (Transformation|SetWorldScale3D _returnvalue_2 "0.800000,0.800000,0.800000")))

(event Custom|Left_Trace
  (bind _rightfist (Variables|Default|GetRightFist))
  (bind _returnvalue (Transformation|GetWorldLocation _rightfist))
  ;[1 1 1] Left
  (bind _outhit (Collision|SphereTraceForObjects _returnvalue (+ _returnvalue (* (Math|Vector|GetForwardVector (Transformation|GetWorldRotation _rightfist)) 3e+02)) 1.5e+02 (Utilities|Array|MakeArray "ObjectTypeQuery3") false 0 "None"))
  (if (== (.HitActor (Collision|BreakHitResult _outhit)) (Game|GetPlayerCharacter 0))
    (bind _returnvalue_2 (Effects|SpawnEmitteratLocation "/Game/Enemies/Blueprints/Anim_Montage_2/P_Spark.P_Spark" (.Location (Collision|BreakHitResult _outhit))))
    (Transformation|SetWorldScale3D _returnvalue_2 "0.800000,0.800000,0.800000")))

(event Custom|DIstancePlayer
  ;[1 1 1] Basic Movement
  (Utilities|Time|SetTimerbyFunctionName 0 "Player Distance" 1.5 true))

(event Custom|Launcher
  (bind _charactermovement (Variables|Character|GetCharacterMovement))
  ;[1 1 1] Launch Character
  (Variables|/Script/Engine.CharacterMovementComponent|SetGroundFriction _charactermovement 0.0)
  (Character|LaunchCharacter (+ (* (Transformation|GetActorForwardVector) (Variables|Default|GetLaunch%20Force)) (* (Transformation|GetActorRightVector) (Variables|Default|GetJump%20Force))) true false)
  (Utilities|FlowControl|RetriggerableDelay 2.5)
  (Variables|/Script/Engine.CharacterMovementComponent|SetGroundFriction _charactermovement 8.0))

(event Custom|LongRange
  ;[1 1 1] Determining Attack
  (Variables|Default|SetIsAttacking true)
  (switch int (Math|Random|RandomIntegerinRange 0 1)
    (:0
      (Variables|Default|SetAnim_Montage "/Game/Enemies/Blueprints/Anim_Montage_2/ExoGame_Troll_Aggro_Montage.ExoGame_Troll_Aggro_Montage"))
    (:1
      (Variables|Default|SetAnim_Montage "/Game/Enemies/Blueprints/Anim_Montage_2/ExoGame_Troll_Attack_Charge_Montage.ExoGame_Troll_Attack_Charge_Montage")
      (Variables|Default|SetLaunch%20Force 1.25e+03)
      (Variables|Default|SetminDmg 12.0)
      (Variables|Default|SetmaxDmg 3e+01)))
  (bind _returnvalue (Animation|PlayAnimMontage (Variables|Default|GetAnim_Montage) 1.0 "None"))
  (Utilities|FlowControl|Delay _returnvalue)
  (Variables|Default|SetIsAttacking false)
  (CallFunction|SeekPlayer)
  (if (<= (Variables|Default|GetDistance) 4e+02)
    (CallFunction|FacePlayer)))

(event Custom|SeekPlayer
  ;[1 1 1] Basic Movement
  (if (Variables|Default|GetIsAttacking)
    (Components|Movement|StopMovementImmediately (Variables|Character|GetCharacterMovement))
    (elif (Variables|Default|GetEnemy_Alive)
      (if (not (Variables|Default|GetFlinch))
        (AI|AIMoveTo self "0, 0, 0" (Game|GetPlayerCharacter 0) 2e+02 false
          (:then
            _)
          (:OnSuccess
            _)
          (:OnFail
            _))
        (Utilities|FlowControl|Delay 0.2)
        (CallFunction|SeekPlayer)))))

(event Custom|Face%20Player
  ;[1 1 1] Rotation
  (Transformation|SetActorRotation (Math|Rotator|FindLookatRotation (Transformation|GetActorLocation) (Transformation|GetActorLocation (Game|GetPlayerCharacter 0)))))

(event Custom|MidRange
  ;[1 1 1] Determining Attack
  (Variables|Default|SetIsAttacking true)
  (switch int (Math|Random|RandomIntegerinRange 0 2)
    (:0
      (Variables|Default|SetAnim_Montage "/Game/Enemies/Blueprints/Anim_Montage_2/ExoGame_Troll_Attack_Charge_Montage.ExoGame_Troll_Attack_Charge_Montage")
      (Variables|Default|SetLaunch%20Force 1.25e+03)
      (Variables|Default|SetminDmg 12.0)
      (Variables|Default|SetmaxDmg 3e+01))
    (:1
      (Variables|Default|SetAnim_Montage "/Game/Enemies/Blueprints/Anim_Montage_2/ExoGame_Troll_Attack_Montage.ExoGame_Troll_Attack_Montage")
      (Variables|Default|SetLaunch%20Force 3e+02)
      (Variables|Default|SetminDmg 15.0)
      (Variables|Default|SetmaxDmg 2e+01))
    (:2
      (Variables|Default|SetAnim_Montage "/Game/Enemies/Blueprints/Anim_Montage_2/ExoGame_Troll_Attack_B_Montage.ExoGame_Troll_Attack_B_Montage")
      (Variables|Default|SetLaunch%20Force 2.5e+02)
      (Variables|Default|SetminDmg 12.0)
      (Variables|Default|SetmaxDmg 2e+01)))
  (bind _returnvalue (Animation|PlayAnimMontage (Variables|Default|GetAnim_Montage) 1.0 "None"))
  (Utilities|FlowControl|Delay _returnvalue)
  (Variables|Default|SetIsAttacking false)
  (CallFunction|SeekPlayer)
  (if (<= (Variables|Default|GetDistance) 4e+02)
    (CallFunction|FacePlayer)))

(event Custom|ShortRange
  ;[1 1 1] Determining Attack
  (Variables|Default|SetIsAttacking true)
  (switch int (Math|Random|RandomIntegerinRange 0 1)
    (:0
      (Variables|Default|SetAnim_Montage "/Game/Enemies/Blueprints/Anim_Montage_2/ExoGame_Troll_Attack_C_Montage.ExoGame_Troll_Attack_C_Montage")
      (Variables|Default|SetLaunch%20Force 3e+02)
      (Variables|Default|SetminDmg 3e+01)
      (Variables|Default|SetmaxDmg 4e+01))
    (:1
      (Variables|Default|SetAnim_Montage "/Game/Enemies/Blueprints/Anim_Montage_2/ExoGame_Troll_Attack_HandSwipe_Montage.ExoGame_Troll_Attack_HandSwipe_Montage")
      (Variables|Default|SetLaunch%20Force 5e+02)
      (Variables|Default|SetminDmg 25.0)
      (Variables|Default|SetmaxDmg 3e+01)))
  (bind _returnvalue (Animation|PlayAnimMontage (Variables|Default|GetAnim_Montage) 1.0 "None"))
  (Utilities|FlowControl|Delay _returnvalue)
  (Variables|Default|SetIsAttacking false)
  (CallFunction|SeekPlayer)
  (if (<= (Variables|Default|GetDistance) 4e+02)
    (CallFunction|FacePlayer)))

(event Custom|dCol_Left_Fist
  ;[1 1 1] Fist Collision
  (Collision|SetCollisionEnabled (Variables|Default|GetLeftFist) "NoCollision"))

(event Custom|eCol_Left_Fist
  ;[1 1 1] Fist Collision
  (Collision|SetCollisionEnabled (Variables|Default|GetLeftFist) "QueryAndPhysics"))

(event Custom|eCol_Right_Fist
  ;[1 1 1] Fist Collision
  (Collision|SetCollisionEnabled (Variables|Default|GetRightFist) "QueryAndPhysics"))

(event Custom|dCol_Right_Fist
  ;[1 1 1] Fist Collision
  (Collision|SetCollisionEnabled (Variables|Default|GetRightFist) "NoCollision"))

(event Game|Damage|EventAnyDamage
  (params (Damage :type Float%20%28single-precision%29) (DamageType :type Damage%20Type%20Object%20Reference) (InstigatedBy :type Controller%20Object%20Reference) (DamageCauser :type Actor%20Object%20Reference))
  ;[1 1 1] Damage and Health
  (Variables|Default|SetHealth (- (Variables|Default|GetHealth) Damage))
  (Development|PrintString "Hello World")
  (if (<= (Variables|Default|GetHealth) 0.0)
    (Utilities|FlowControl|DoOnce false
      (:Completed
        (Game|SpawnActorfromClass "/Game/Blueprints/Particle/Death_Particles.Death_Particles_C" (Math|Conversions|ToTransform(Vector) (Transformation|GetSocketLocation (Variables|Character|GetMesh) "head")) "Undefined" 0 0)
        (Variables|Default|SetAnim_Montage "/Game/Enemies/Blueprints/Anim_Montage_2/ExoGame_Troll_React_Death_Montage.ExoGame_Troll_React_Death_Montage")
        (Animation|PlayAnimMontage (Variables|Default|GetAnim_Montage) 1.0 "None")
        (Variables|Default|SetEnemy_Alive false)
        (Utilities|FlowControl|Delay 3.0)
        (Actor|DestroyActor)))
    (else
      (Variables|Default|SetAcc_Dmg (+ Damage (Variables|Default|GetAcc_Dmg)))
      (Utilities|FlowControl|RetriggerableDelay 1.0)
      (Variables|Default|SetAcc_Dmg 0.0)
      (if (>= (Variables|Default|GetAcc_Dmg) 8.0)
        (switch int (Math|Random|RandomIntegerinRange 0 1)
          (:0
            (Variables|Default|SetAnim_Montage "/Game/Enemies/Blueprints/Anim_Montage_2/ExoGame_Troll_React_Heavy_Front_Montage.ExoGame_Troll_React_Heavy_Front_Montage"))
          (:1
            (Variables|Default|SetAnim_Montage "/Game/Enemies/Blueprints/Anim_Montage_2/ExoGame_Troll_React_KnowckBack_Front_Montage.ExoGame_Troll_React_KnowckBack_Front_Montage")))
        (Animation|PlayAnimMontage 0 1.0 "None")
        (Variables|Default|SetFlinch true)))))

(event EventBeginPlay
  ;[1 1 1] Basic Movement
  ;[1 1 1] Initialize
  (Variables|Default|SetHealth 1e+01)
  (Variables|Default|SetEnemy_Alive false)
  (Variables|Default|SetFlinch false)
  (Utilities|FlowControl|Delay 0.2)
  (CallFunction|SeekPlayer)
  (CallFunction|DIstancePlayer))

(fn ConstructionScript)

(fn PlayerDistance
  ;[1 1 1] Calculate Distance
  (if (not (Variables|Default|GetIsAttacking))
    (bind _output_get (Variables|Default|SetDistance (Math|Vector|VectorLength (- (Transformation|GetActorLocation) (Transformation|GetActorLocation (Game|GetPlayerCharacter 0))))))
    ;[1 1 1] Determining Attacks
    (if (and (>= _output_get 4.5e+02) (<= _output_get 2e+03))
      ;[1 1 1] Run Attacks
      (Development|PrintString "a3")
      (if (== (Math|Random|RandomIntegerinRange 0 2) 0)
        (CallFunction|LongRange)
        (else
          (CallFunction|SeekPlayer)))
      (elif (>= _output_get 301.0)
        (Development|PrintString "a2")
        (CallFunction|MidRange)
        (elif (<= _output_get 3e+02)
          (Development|PrintString "Hi There")
          (CallFunction|ShortRange))))))