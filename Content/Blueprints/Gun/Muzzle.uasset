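; Muzzle is a short-lived actor that spawns Bullet actors when a gun fires, then destroys itself.
; BulletFire stores the gun properties and transform, passes through a gate opened on BeginPlay, and switches on gun type.
; Crossbow, lance and pistol each spawn one bullet at the given transform, while the shotgun spawns several with random pitch and yaw bloom.
; Each bullet receives the gun type.
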(event Custom|BulletFire
  (params (Gun_Properties :type Gun%20Properties%20Structure) (Location :type Transform))
  (bind _output_get (Variables|Default|SetGun_Properties Gun_Properties))
  (Variables|Default|SetLocation Location)
  (Utilities|FlowControl|Gate true
    (:Exit
      (switch Utilities|FlowControl|Switch|SwitchonGun_Type (.Gun_Type (Utilities|Struct|BreakGun_Properties _output_get))
        (:NewEnumerator0
          ;[1 1 1] Crossbow
          (Game|SpawnActorfromClass "/Game/Blueprints/Gun/Bullet.Bullet_C" (Variables|Default|GetLocation) "Undefined" 0 (.Gun_Type (Utilities|Struct|BreakGun_Properties _output_get)) 0))
        (:NewEnumerator2
          ;[1 1 1] Lance
          (Game|SpawnActorfromClass "/Game/Blueprints/Gun/Bullet.Bullet_C" (Variables|Default|GetLocation) "Undefined" 0 (.Gun_Type (Utilities|Struct|BreakGun_Properties _output_get)) 0))
        (:NewEnumerator1
          ;[1 1 1] Pistol
          (Game|SpawnActorfromClass "/Game/Blueprints/Gun/Bullet.Bullet_C" (Variables|Default|GetLocation) "Undefined" 0 (.Gun_Type (Utilities|Struct|BreakGun_Properties _output_get)) 0))
        (:NewEnumerator3
          ;[1 1 1] Shotgun
          (for _index (range 0 5)
            (Game|SpawnActorfromClass "/Game/Blueprints/Gun/Bullet.Bullet_C" (Math|Transform|MakeTransform (.Location (Math|Transform|BreakTransform (Variables|Default|GetLocation))) (Math|Rotator|MakeRotator (.Roll (Math|Rotator|BreakRotator (.Rotation (Math|Transform|BreakTransform (Variables|Default|GetLocation))))) (+ (Math|Random|RandomFloatinRange (Variables|Default|GetBloom) (Variables|Default|GetNBloom)) (.Pitch (Math|Rotator|BreakRotator (.Rotation (Math|Transform|BreakTransform (Variables|Default|GetLocation)))))) (+ (Math|Random|RandomFloatinRange (Variables|Default|GetBloom) (Variables|Default|GetNBloom)) (.Yaw (Math|Rotator|BreakRotator (.Rotation (Math|Transform|BreakTransform (Variables|Default|GetLocation))))))) (.Scale (Math|Transform|BreakTransform (Variables|Default|GetLocation)))) "Undefined" 0 (.Gun_Type (Utilities|Struct|BreakGun_Properties _output_get)) 0))))
      (Actor|DestroyActor))))

(event EventBeginPlay
  (bind _location (Variables|Default|GetLocation))
  (bind _location_2 (Variables|Default|GetLocation))
  (bind (_location_3 _rotation _scale) (Math|Transform|BreakTransform _location_2))
  (bind _rotation_2 (Math|Transform|BreakTransform _location))
  (bind (_roll _pitch _yaw) (Math|Rotator|BreakRotator _rotation_2))
  (Utilities|FlowControl|Gate true) ; enters at Open
)

(event Collision|EventActorBeginOverlap
  (params (OtherActor :type Actor%20Object%20Reference)))

(event EventTick
  (params (DeltaSeconds :type Float%20%28single-precision%29)))

(fn ConstructionScript)